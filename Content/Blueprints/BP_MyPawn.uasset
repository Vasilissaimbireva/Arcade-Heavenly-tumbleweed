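; Arcade game pawn that handles heart bonus pickups and saves the high score.
; When its collision overlaps a heart bonus, it calls ChangeHealths with 1 on the game mode's health component if health is below the cap.
; On EndPlay it loads or creates the high-score save slot, writing the game mode's points when no save exists or the stored record is beaten.
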(event `self.PawnCollision.OnComponentBeginOverlap`
  (params (OverlappedComponent :type "PrimitiveComponent Object Reference") (OtherActor :type "Actor Object Reference") (OtherComp :type "PrimitiveComponent Object Reference") (OtherBodyIndex :type Integer) (bFromSweep :type Boolean) (SweepResult :type "HitResult Structure (by ref)"))
  (cast `/Game/Blueprints/BP_Bonus_heart` OtherActor)
  (bind _asbp_arcade_1game_mode (cast `/Game/Blueprints/BP_Arcade1GameMode` (`GameplayStatics.GetGameMode`)))
  (if (< (`GameHealthComponent.GetHealths` (`StremArcade1GameModeBase.HealthsComponent` _asbp_arcade_1game_mode)) 5)
    (bind _asbp_arcade_1game_mode_2 (cast `/Game/Blueprints/BP_Arcade1GameMode` (`GameplayStatics.GetGameMode`)))
    (bind _returnvalue (`GameHealthComponent.GetHealths` (`StremArcade1GameModeBase.HealthsComponent` _asbp_arcade_1game_mode_2)))
    (`GameHealthComponent.ChangeHealths` (`StremArcade1GameModeBase.HealthsComponent` _asbp_arcade_1game_mode_2) (+ (- _returnvalue _returnvalue) 1))))

(event `self.ReceiveEndPlay`
  (params (EndPlayReason :type "EEndPlayReason Enum" :default "Destroyed"))
  (bind _savesubclass (`self.SaveSubClass`))
  (bind _asbp_arcade_1game_mode (cast `/Game/Blueprints/BP_Arcade1GameMode` (`GameplayStatics.GetGameMode`)))
  (bind _returnvalue (`GameplayStatics.DoesSaveGameExist` "HighsCoreData"))
  (if _returnvalue
    (bind _returnvalue_2 (`GameplayStatics.LoadGameFromSlot` "HighsCoreData"))
    (bind _output_get (set `self.SaveSubClass` _returnvalue_2))
    (bind _asbp_save_game (cast `/Game/Save/BP_SaveGame` _output_get))
    (bind _gamepoints (`StremArcade1GameModeBase.GamePoints` _asbp_arcade_1game_mode))
    (if (> _gamepoints (`/Game/Save/BP_SaveGame.HighsCoreValue` _asbp_save_game))
      (set `/Game/Save/BP_SaveGame.HighsCoreValue` _gamepoints _asbp_save_game)
      (`GameplayStatics.SaveGameToSlot` _savesubclass "HighsCoreData"))
    (else
      (bind _returnvalue_3 (`GameplayStatics.CreateSaveGameObject` "/Game/Save/BP_SaveGame.BP_SaveGame_C"))
      (bind _output_get_2 (set `self.SaveSubClass` _returnvalue_3))
      (bind _asbp_save_game_2 (cast `/Game/Save/BP_SaveGame` _output_get_2))
      (set `/Game/Save/BP_SaveGame.HighsCoreValue` _gamepoints _asbp_save_game_2)
      (`GameplayStatics.SaveGameToSlot` _savesubclass "HighsCoreData"))))

(fn `UserConstructionScript`)