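; BP_BaseEnemy_4 is an enemy actor that constantly moves forward while gradually homing in on the player pawn cached at BeginPlay.
; Each Tick it advances along its local X axis by a fixed step that is not scaled by delta time, with no sweep.
; It yaws toward the player using the clamped look-at angle difference scaled by delta time, giving a capped, proportional turn rate.
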(event `self.ReceiveBeginPlay`
  (`parent.ReceiveBeginPlay`)
  (set `self.MP` (`GameplayStatics.GetPlayerPawn` 0)))

(event `self.ReceiveTick`
  (params (DeltaSeconds :type "Float (single-precision)"))
  (bind (_returnvalue_roll _returnvalue_pitch _returnvalue_yaw) (`KismetMathLibrary.BreakRotator` (`KismetMathLibrary.NormalizedDeltaRotator` (`KismetMathLibrary.FindLookAtRotation` (`self.K2_GetActorLocation`) (`self.K2_GetActorLocation` (`self.MP`))) (`self.K2_GetActorRotation`))))
  (`parent.ReceiveTick` DeltaSeconds)
  (`self.K2_AddActorLocalOffset` (5.0 0.0 0.0))
  (`self.MP`
    (:`then`
      (`self.K2_AddActorLocalRotation` (`KismetMathLibrary.MakeRotator` 0.0 0.0 (* (`KismetMathLibrary.FClamp` _returnvalue_yaw -35.0 35.0) (`GameplayStatics.GetWorldDeltaSeconds`)))))
    (:`else`)))

(fn `UserConstructionScript`)